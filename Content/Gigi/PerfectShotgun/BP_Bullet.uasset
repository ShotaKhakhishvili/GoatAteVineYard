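; BP_Bullet is a shotgun projectile that damages fighter characters it overlaps and destroys itself after five seconds.
; Its sphere overlap runs DecideToDamage, which requires the hitting flag, skips the owner and accepts only BP_FighterCharacter targets.
; With a valid owner ability, damage is scaled by that ability's attitude toward the target's ability type, then a random hit sound and cloud Niagara effect play.
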(event OnComponentBeginOverlap(Sphere)
  (params (OverlappedComponent :type Primitive%20Component%20Object%20Reference) (OtherActor :type Actor%20Object%20Reference) (OtherComp :type Primitive%20Component%20Object%20Reference) (OtherBodyIndex :type Integer) (bFromSweep :type Boolean) (SweepResult :type Hit%20Result%20Structure%20%28by%20ref%29))
  (CallFunction|DecidetoDamage OtherActor))

(event EventBeginPlay
  (Utilities|FlowControl|Delay 5.0)
  (Actor|DestroyActor))

(event Collision|EventActorBeginOverlap
  (params (OtherActor :type Actor%20Object%20Reference)))

(event EventTick
  (params (DeltaSeconds :type Float%20%28single-precision%29)))

(fn ConstructionScript)

(fn DecidetoDamage
  (params (OtherActor :type Object%20Object%20Reference))
  (if (Variables|Default|GetItHitting?)
    (if (not (== OtherActor (Variables|Default|GetOwnerActor)))
      (bind _asbp_fighter_character (Utilities|Casting|CastToBP_FighterCharacter OtherActor))
      (Variables|Default|SetLast%20hit%20actor _asbp_fighter_character)
      (Utilities|IsValid (Variables|Default|GetLast%20hit%20actor)
        (:Is%20Valid
          (Utilities|IsValid (Variables|Default|GetOwnerAbility)
            (:Is%20Valid
              (Default|FApplyDamage (Variables|Default|GetLast%20hit%20actor) (* (Variables|Default|GetDamage) (CallFunction|FLGetAttitude (Variables|/Game/Shota/Blueprints/Abilities/BP_Ability.BP_Ability_C|GetType (Variables|/Game/Shota/Blueprints/Fighter/BP_FighterCharacter.BP_FighterCharacter_C|GetAbility (Variables|Default|GetLast%20hit%20actor))) (Variables|/Game/Shota/Blueprints/Abilities/BP_Ability.BP_Ability_C|GetAttitudes (Variables|Default|GetOwnerAbility)))))
              (Audio|PlaySoundatLocation (.OutItem (Utilities|Array|Random (Variables|Default|GetHitSounds))) (Transformation|GetActorLocation) "0, 0, 0" 1.0 1.0 0.0 0 0 0 0)
              (Niagara|SpawnSystematLocation "/Game/Gigi/Explosions/NS_NormalClouds.NS_NormalClouds" (Transformation|GetActorLocation)))))))))