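; BP_Territory is a spherical animal territory that populates itself with its owner species and watches for intruders of other species.
; On BeginPlay it spawns NAnimals at random reachable navmesh points within the sphere, linking each to the territory and its own AI controller.
; Sphere overlaps tag intruding fighter characters with the territory ID, clearing it on exit, and maintain an enemy count and presence flag.
; IsPointInsideDomain is a stub returning false.
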(event OnComponentBeginOverlap(Sphere)
  (params (OverlappedComponent :type Primitive%20Component%20Object%20Reference) (OtherActor :type Actor%20Object%20Reference) (OtherComp :type Primitive%20Component%20Object%20Reference) (OtherBodyIndex :type Integer) (bFromSweep :type Boolean) (SweepResult :type Hit%20Result%20Structure%20%28by%20ref%29))
  (if (!= (Utilities|GetClass OtherActor) (Variables|Default|GetOwnerSpecies))
    (bind _asbp_fighter_character (Utilities|Casting|CastToBP_FighterCharacter OtherActor))
    (Variables|/Game/Shota/Blueprints/Fighter/BP_FighterCharacter.BP_FighterCharacter_C|SetInTerritoryID _asbp_fighter_character (Variables|Default|GetID))
    (Math|Integer|IncrementInt (Variables|Default|GetnEnemies)
      (:%20%20
        (Variables|Default|SetEnemyInTerritory? true)))))

(event OnComponentEndOverlap(Sphere)
  (params (OverlappedComponent :type Primitive%20Component%20Object%20Reference) (OtherActor :type Actor%20Object%20Reference) (OtherComp :type Primitive%20Component%20Object%20Reference) (OtherBodyIndex :type Integer))
  (if (!= (Utilities|GetClass OtherActor) (Variables|Default|GetOwnerSpecies))
    (bind _asbp_fighter_character (Utilities|Casting|CastToBP_FighterCharacter OtherActor))
    (Variables|/Game/Shota/Blueprints/Fighter/BP_FighterCharacter.BP_FighterCharacter_C|SetInTerritoryID _asbp_fighter_character -1)
    (bind _result (Math|Integer|DecrementInt (Variables|Default|GetnEnemies))
      (:%20%20
        (if (< _result 1)
          (Variables|Default|SetnEnemies 0)
          (Variables|Default|SetEnemyInTerritory? false))))))

(event EventBeginPlay
  (Variables|Default|SetRadius (Components|Sphere|GetScaledSphereRadius (Variables|Default|GetSphere)))
  (if (not (== (Variables|Default|GetSpawned) (Variables|Default|GetnAnimals))) :!label _label
    (bind _returnvalue (Game|SpawnActorfromClass (Variables|Default|GetOwnerSpecies) (Math|Transform|MakeTransform (.Location (CallFunction|GetRandomPointInsideDomain)) (Math|Rotator|MakeRotator 0.0 0.0 (* (Math|Random|RandomFloat) 1.8e+02))) "AdjustIfPossibleButAlwaysSpawn" "OverrideRootScale" 0 0))
    (Variables|/Game/Shota/Blueprints/Fighter/BP_FighterCharacter.BP_FighterCharacter_C|SetTerritory _returnvalue self)
    (Variables|/Game/Shota/Blueprints/Fighter/BP_FighterCharacter.BP_FighterCharacter_C|SetInTerritoryID _returnvalue (Variables|Default|GetID))
    ;[0.15 0.15 0.15 0.5] CHANGEEE
    (bind _returnvalue_2 (Game|SpawnActorfromClass "/Game/Gigi/AI/BP_BaseAnimalAIController.BP_BaseAnimalAIController_C" (Math|Transform|MakeTransform "0, 0, 0") "AlwaysSpawn" "MultiplyWithRoot" 0 _returnvalue 0))
    (Variables|/Game/Shota/Blueprints/Fighter/BP_FighterCharacter.BP_FighterCharacter_C|SetAIController _returnvalue _returnvalue_2)
    (Math|Integer|IncrementInt (Variables|Default|GetSpawned)
      (:%20%20
        (goto _label)))))

(fn ConstructionScript)

(fn GetRandomPointInsideDomain
  (bind _returnvalue (Transformation|GetActorLocation))
  (bind _radius (Variables|Default|GetRadius))
  (bind (_randomlocation _returnvalue_2) (AI|Navigation|GetRandomReachablePointinRadius _returnvalue _radius 0 0))
  (return (+ _randomlocation "0.000000,0.000000,100.000000") _returnvalue_2))

(fn IsPointInsideDomain
  (params (NewParam :type Vector))
  (return false))