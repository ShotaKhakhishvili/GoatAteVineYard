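; BP_FighterCharacter_Dirt is a Dirt-named fighter character Blueprint in the Gigi bots folder.
; Its BeginPlay, construction script and two AI ability enemy checks only forward to the parent class, so the graphs add no logic of their own.
; Tick is disabled and ActorBeginOverlap is an empty disabled stub, leaving all visible behavior inherited.
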(event Collision|EventActorBeginOverlap
  (params (OtherActor :type Actor%20Object%20Reference)))

(event EventTick
  (params (DeltaSeconds :type Float%20%28single-precision%29))
  (|CallParentFunction DeltaSeconds) ; This node is disabled and will not be called.\nDrag off pins to build functionality.
)

(event EventBeginPlay
  (|CallParentFunction))

(fn ConstructionScript
  (|CallParentFunction))

(fn AISimpleAbilityEnemyCheck
  (return (|CallParentFunction)))

(fn AIAbilityEnemyCheck
  (return (|CallParentFunction)))