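; BP_OptimizationGrid is a trigger volume that switches bots on or off by territory based on the player's location.
; When the player character enters its box, it activates bots in the visible territories and deactivates those in the hidden ones.
; BeginPlay waits two ticks, then runs the same switch if the player already starts inside the box.
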(event OnComponentBeginOverlap(Box)
  (params (OverlappedComponent :type Primitive%20Component%20Object%20Reference) (OtherActor :type Actor%20Object%20Reference) (OtherComp :type Primitive%20Component%20Object%20Reference) (OtherBodyIndex :type Integer) (bFromSweep :type Boolean) (SweepResult :type Hit%20Result%20Structure%20%28by%20ref%29))
  (if (== OtherActor (Game|GetPlayerCharacter 0))
    (for _array_element (Variables|Default|GetVisibleTerritories)
      (Default|ActivateBots _array_element))
    (for _array_element_2 (Variables|Default|GetHiddenTerritories)
      (Default|DeactivateBots _array_element_2))))

(event EventBeginPlay
  (Utilities|FlowControl|DelayUntilNextTick)
  (Utilities|FlowControl|DelayUntilNextTick)
  (if (Collision|IsOverlappingActor (Variables|Default|GetBox) (Game|GetPlayerCharacter 0) :!class /Script/Engine.PrimitiveComponent)
    (for _array_element (Variables|Default|GetVisibleTerritories)
      (Default|ActivateBots _array_element))
    (for _array_element_2 (Variables|Default|GetHiddenTerritories)
      (Default|DeactivateBots _array_element_2))))

(fn ConstructionScript)