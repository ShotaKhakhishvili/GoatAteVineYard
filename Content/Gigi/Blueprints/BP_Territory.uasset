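; Territory actor that populates a spherical area with animals of its owner species and tracks intruders of other classes.
; On BeginPlay it spawns animals with AI controllers at random reachable points until the starting count is met, then deactivates them.
; Sphere overlaps stamp fighters with the territory ID and maintain the enemy count and flag.
; Deaths optionally trigger respawns, and ActivateBots restores the dormant animals' movement, collision, visibility and AI logic.
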(event OnComponentBeginOverlap(Sphere)
  (params (OverlappedComponent :type Primitive%20Component%20Object%20Reference) (OtherActor :type Actor%20Object%20Reference) (OtherComp :type Primitive%20Component%20Object%20Reference) (OtherBodyIndex :type Integer) (bFromSweep :type Boolean) (SweepResult :type Hit%20Result%20Structure%20%28by%20ref%29))
  (CallFunction|CheckEnemies OtherActor))

(event OnComponentEndOverlap(Sphere)
  (params (OverlappedComponent :type Primitive%20Component%20Object%20Reference) (OtherActor :type Actor%20Object%20Reference) (OtherComp :type Primitive%20Component%20Object%20Reference) (OtherBodyIndex :type Integer))
  (if (not (== (Utilities|GetClass OtherActor) (Variables|Default|GetOwnerSpecies)))
    (bind _asbp_fighter_character (Utilities|Casting|CastToBP_FighterCharacter OtherActor))
    (Variables|/Game/Shota/Blueprints/Fighter/BP_FighterCharacter.BP_FighterCharacter_C|SetInTerritoryID _asbp_fighter_character -1)
    (bind _result (Math|Integer|DecrementInt (Variables|Default|GetnEnemies))
      (:%20%20
        (if (< _result 1)
          (Variables|Default|SetnEnemies 0)
          (Variables|Default|SetEnemyInTerritory? false))))))

(event Custom|CharacterDied
  (params (DeadCharacter :type BP%20Fighter%20Character%20Object%20Reference))
  (Math|Integer|DecrementInt (Variables|Default|GetAliveAnimals)
    (:%20%20
      (Utilities|Array|RemoveItem (Variables|Default|GetMyAnimals) DeadCharacter)
      (if (Variables|Default|GetRespawnBots?)
        (CallFunction|SpawnOneGuy)))))

(event Custom|CheckEnemies
  (params (Actor :type Object%20Object%20Reference))
  (if (== (Utilities|GetClass Actor) (Variables|Default|GetOwnerSpecies))
    (bind _asbp_fighter_character (Utilities|Casting|CastToBP_FighterCharacter Actor))
    (Variables|/Game/Shota/Blueprints/Fighter/BP_FighterCharacter.BP_FighterCharacter_C|SetInTerritoryID _asbp_fighter_character (Variables|Default|GetID))
    (else
      (bind _asbp_fighter_character_2 (Utilities|Casting|CastToBP_FighterCharacter Actor))
      (Variables|/Game/Shota/Blueprints/Fighter/BP_FighterCharacter.BP_FighterCharacter_C|SetInTerritoryID _asbp_fighter_character_2 (Variables|Default|GetID))
      (Math|Integer|IncrementInt (Variables|Default|GetnEnemies)
        (:%20%20
          (Variables|Default|SetEnemyInTerritory? true))))))

(event EventBeginPlay
  (Variables|Default|SetRadius (Components|Sphere|GetScaledSphereRadius (Variables|Default|GetSphere)))
  (Utilities|FlowControl|DelayUntilNextTick)
  (if (== (Variables|Default|GetAliveAnimals) (Variables|Default|GetnStartingAnimals)) :!label _label
    (CallFunction|DeactivateBots)
    (for _array_element (Collision|GetOverlappingActors "/Game/Shota/Blueprints/Fighter/BP_FighterCharacter.BP_FighterCharacter_C" :!class /Script/Engine.Actor)
      (CallFunction|CheckEnemies _array_element))
    (else
      (CallFunction|SpawnOneGuy)
      (goto _label))))

(fn ConstructionScript)

(fn GetRandomPointInsideDomain
  (bind _returnvalue (Transformation|GetActorLocation))
  (bind _radius (Variables|Default|GetRadius))
  (bind (_randomlocation _returnvalue_2) (AI|Navigation|GetRandomReachablePointinRadius _returnvalue _radius 0 0))
  (return (+ _randomlocation "0.000000,0.000000,100.000000") _returnvalue_2))

(fn IsPointInsideDomain
  (params (NewParam :type Vector))
  (return false))

(fn SpawnOneGuy
  (bind _returnvalue (Game|SpawnActorfromClass (Variables|Default|GetOwnerSpecies) (Math|Transform|MakeTransform (.Location (CallFunction|GetRandomPointInsideDomain)) (Math|Rotator|MakeRotator 0.0 0.0 (* (Math|Random|RandomFloat) 1.8e+02))) "AdjustIfPossibleButAlwaysSpawn" "OverrideRootScale" 0 (Variables|Default|GetID) 0))
  (bind _output_get (LocalVariables|SetActor _returnvalue))
  (Utilities|Array|Add (Variables|Default|GetMyAnimals) _output_get)
  (Variables|/Game/Shota/Blueprints/Fighter/BP_FighterCharacter.BP_FighterCharacter_C|SetTerritory (LocalVariables|GetActor) self)
  (bind _returnvalue_2 (Game|SpawnActorfromClass "/Game/Gigi/AI/BP_BaseAnimalAIController.BP_BaseAnimalAIController_C" (Math|Transform|MakeTransform "0, 0, 0") "AlwaysSpawn" "MultiplyWithRoot" 0 (LocalVariables|GetActor) (Variables|Default|GetID) 0))
  (LocalVariables|SetControler _returnvalue_2)
  (Variables|/Game/Shota/Blueprints/Fighter/BP_FighterCharacter.BP_FighterCharacter_C|SetAIController (LocalVariables|GetActor) (LocalVariables|GetControler))
  (Math|Integer|IncrementInt (Variables|Default|GetAliveAnimals)
    (:%20%20
      (return))))

(fn DeactivateBots
  (for _array_element (Variables|Default|GetMyAnimals)
    (Components|Activation|Deactivate (Variables|/Script/Engine.Character|GetCharacterMovement _array_element))
    (Collision|SetActorEnableCollision _array_element false)
    (Components|Tick|SetComponentTickEnabled (Variables|/Script/Engine.Character|GetMesh _array_element) false)
    (Rendering|SetActorHiddenInGame _array_element true)
    (AI|Logic|StopLogic (Variables|/Script/AIModule.AIController|GetBrainComponent (Variables|/Game/Shota/Blueprints/Fighter/BP_FighterCharacter.BP_FighterCharacter_C|GetAIController _array_element)) "NoNeed"))
  (return))

(fn ActivateBots
  (for _array_element (Variables|Default|GetMyAnimals)
    (Components|Activation|Activate (Variables|/Script/Engine.Character|GetCharacterMovement _array_element) true)
    (Collision|SetActorEnableCollision _array_element true)
    (Components|Tick|SetComponentTickEnabled (Variables|/Script/Engine.Character|GetMesh _array_element) true)
    (Rendering|SetActorHiddenInGame _array_element false)
    (AI|Logic|StartLogic (Variables|/Script/AIModule.AIController|GetBrainComponent (Variables|/Game/Shota/Blueprints/Fighter/BP_FighterCharacter.BP_FighterCharacter_C|GetAIController _array_element))))
  (return))