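; BP_Grape is a pickup-style actor that can finish the game when the player touches it with the Messi ability.
; On BeginPlay it caches player 0's BP_FighterCharacter_Player.
; When its Sphere starts overlapping that player, it checks that the player's Ability is exactly BP_Ability_Messi, then casts the game instance to BP_FinishedGame and calls Finished.
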(event OnComponentBeginOverlap(Sphere)
  (params (OverlappedComponent :type Primitive%20Component%20Object%20Reference) (OtherActor :type Actor%20Object%20Reference) (OtherComp :type Primitive%20Component%20Object%20Reference) (OtherBodyIndex :type Integer) (bFromSweep :type Boolean) (SweepResult :type Hit%20Result%20Structure%20%28by%20ref%29))
  (if (== OtherActor (Variables|Default|GetPlayer))
    (if (== (Utilities|GetClass (Variables|/Game/Shota/Blueprints/Fighter/BP_FighterCharacter.BP_FighterCharacter_C|GetAbility (Variables|Default|GetPlayer))) "/Game/Shota/Blueprints/Abilities/BP_Ability_Messi.BP_Ability_Messi_C")
      (bind _asbp_finished_game (Utilities|Casting|CastToBP_FinishedGame (Game|GetGameInstance)))
      (Default|Finished _asbp_finished_game))))

(event Collision|EventActorBeginOverlap
  (params (OtherActor :type Actor%20Object%20Reference)))

(event EventTick
  (params (DeltaSeconds :type Float%20%28single-precision%29)))

(event EventBeginPlay
  (bind _asbp_fighter_character_player (Utilities|Casting|CastToBP_FighterCharacter_Player (Game|GetPlayerCharacter 0)))
  (Variables|Default|SetPlayer _asbp_fighter_character_player))

(fn ConstructionScript)