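; AI controller for animal fighter characters that runs the BT_BaseAnimal behavior tree and seeds its blackboard on BeginPlay.
; It caches the controlled fighter, possessing a preset one if needed, and writes self and the shorter of two ability ranges.
; A valid Territory enables Patrol and supplies its location, radius and an ID.
; SetEnemy writes or clears the Enemy key and sets focus on the controller's own fighter when the enemy is valid.
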(event Custom|SetEnemy
  (params (Enemy :type BP%20Fighter%20Character%20Object%20Reference))
  (Utilities|IsValid Enemy
    (:Is%20Valid
      (AI|SetFocus (Variables|Default|GetOwnerFighterChar))
      (AI|Components|Blackboard|SetValueasObject (AI|GetBlackboard 0) (Utilities|Name|MakeLiteralName "Enemy") Enemy)
      (AI|Components|Blackboard|SetValueasVector (Variables|Default|GetAnimalBlackBoard) (Utilities|Name|MakeLiteralName "EnemyLocation") (Transformation|GetActorLocation Enemy)))
    (:Is%20Not%20Valid
      (AI|Components|Blackboard|ClearValue (AI|GetBlackboard 0) (Utilities|Name|MakeLiteralName "Enemy")))))

(event EventBeginPlay
  (bind _asbp_fighter_character (Utilities|Casting|CastToBP_FighterCharacter (Pawn|GetControlledPawn))
    (:then
      (Variables|Default|SetOwnerFighterChar _asbp_fighter_character))
    (:CastFailed
      (Utilities|IsValid (Variables|Default|GetOwnerFighterChar)
        (:Is%20Valid
          (Pawn|Possess (Variables|Default|GetOwnerFighterChar))))))
  (AI|RunBehaviorTree "/Game/Gigi/AI/BT_BaseAnimal.BT_BaseAnimal")
  (Variables|Default|SetAnimalBlackBoard (AI|GetBlackboard 0))
  (AI|Components|Blackboard|SetValueasObject (AI|GetBlackboard 0) (Utilities|Name|MakeLiteralName "SelfActor") (Variables|Default|GetOwnerFighterChar))
  (AI|Components|Blackboard|SetValueasFloat (AI|GetBlackboard 0) (Utilities|Name|MakeLiteralName "AbilityDistance") (Math|Float|Min(Float) (Variables|/Game/Shota/Blueprints/Abilities/BP_Ability.BP_Ability_C|GetSimpleAbilityCloseDistance (Variables|/Game/Shota/Blueprints/Fighter/BP_FighterCharacter.BP_FighterCharacter_C|GetAbility (Variables|Default|GetOwnerFighterChar))) (Variables|/Game/Shota/Blueprints/Abilities/BP_Ability.BP_Ability_C|GetAbilityCloseDistance (Variables|/Game/Shota/Blueprints/Fighter/BP_FighterCharacter.BP_FighterCharacter_C|GetAbility (Variables|Default|GetOwnerFighterChar)))))
  (Utilities|IsValid (Variables|/Game/Shota/Blueprints/Fighter/BP_FighterCharacter.BP_FighterCharacter_C|GetTerritory (Variables|Default|GetOwnerFighterChar))
    (:Is%20Valid
      (Variables|Default|SetTerritory (Variables|/Game/Shota/Blueprints/Fighter/BP_FighterCharacter.BP_FighterCharacter_C|GetTerritory (Variables|Default|GetOwnerFighterChar)))
      (Variables|Default|SetTerritoryRadius (Variables|/Game/Gigi/BP_Territory.BP_Territory_C|GetRadius (Variables|/Game/Shota/Blueprints/Fighter/BP_FighterCharacter.BP_FighterCharacter_C|GetTerritory (Variables|Default|GetOwnerFighterChar))))
      (AI|Components|Blackboard|SetValueasBool (Variables|Default|GetAnimalBlackBoard) (Utilities|Name|MakeLiteralName "Patrol") true)
      (AI|Components|Blackboard|SetValueasObject (Variables|Default|GetAnimalBlackBoard) (Utilities|Name|MakeLiteralName "Territory") (Variables|/Game/Shota/Blueprints/Fighter/BP_FighterCharacter.BP_FighterCharacter_C|GetTerritory (Variables|Default|GetOwnerFighterChar)))
      (AI|Components|Blackboard|SetValueasVector (Variables|Default|GetAnimalBlackBoard) (Utilities|Name|MakeLiteralName "TerritoryLocation") (Transformation|GetActorLocation (Variables|Default|GetTerritory)))
      (AI|Components|Blackboard|SetValueasFloat (AI|GetBlackboard 0) (Utilities|Name|MakeLiteralName "TerritoryRadius") (Variables|Default|GetTerritoryRadius))
      (Class|BlackboardComponent|SetValueasInt (AI|GetBlackboard 0) (Utilities|Name|MakeLiteralName "TerritoryID") (Variables|Default|GetID)))
    (:Is%20Not%20Valid
      (AI|Components|Blackboard|SetValueasBool (Variables|Default|GetAnimalBlackBoard) (Utilities|Name|MakeLiteralName "Patrol") false))))

(fn ConstructionScript)