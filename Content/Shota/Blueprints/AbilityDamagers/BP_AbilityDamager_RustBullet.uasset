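; Projectile ability damager for the Rust bullet, which damages fighters whose ability type differs from its owner's.
; On sphere overlap it scales damage by the owner ability's attitude toward the target's type, while same-type fighters are ignored.
; Damaging hits and overlaps with other non-fighter actors fire the on-hit call.
; The first hit also removes the collision sphere, stops movement and shrinks the bullet by timeline before destroying it.
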(event OnComponentBeginOverlap(Sphere)
  (params (OverlappedComponent :type Primitive%20Component%20Object%20Reference) (OtherActor :type Actor%20Object%20Reference) (OtherComp :type Primitive%20Component%20Object%20Reference) (OtherBodyIndex :type Integer) (bFromSweep :type Boolean) (SweepResult :type Hit%20Result%20Structure%20%28by%20ref%29))
  (bind _asbp_fighter_character (Utilities|Casting|CastToBP_FighterCharacter OtherActor)
    (:then
      (if (Utilities|Enum|NotEqual(Enum) (Variables|/Game/Shota/Blueprints/Abilities/BP_Ability.BP_Ability_C|GetType (Variables|/Game/Shota/Blueprints/Fighter/BP_FighterCharacter.BP_FighterCharacter_C|GetAbility _asbp_fighter_character)) (Variables|/Game/Shota/Blueprints/Abilities/BP_Ability.BP_Ability_C|GetType (Variables|Default|GetOwnerAbility)))
        (Default|FApplyDamage _asbp_fighter_character (* (Variables|Default|GetDamage) (CallFunction|FLGetAttitude (Variables|/Game/Shota/Blueprints/Abilities/BP_Ability.BP_Ability_C|GetType (Variables|/Game/Shota/Blueprints/Fighter/BP_FighterCharacter.BP_FighterCharacter_C|GetAbility _asbp_fighter_character)) (Variables|/Game/Shota/Blueprints/Abilities/BP_Ability.BP_Ability_C|GetAttitudes (Variables|Default|GetOwnerAbility)))))
        (Default|CallOnHit :!label _label)
        (Utilities|FlowControl|DoOnce false
          (:Completed
            (Components|DestroyComponent (Variables|Default|GetSphere))
            (Variables|/Script/Engine.ProjectileMovementComponent|SetbSimulationEnabled (Variables|Default|GetProjectileMovement) false)
            (bind _size (Timeline|ShrinkToDeath PlayFromStart)
              (:Update
                (Transformation|SetActorScale3D (Math|Conversions|ToVector(Float) _size)))
              (:Finished
                (Actor|DestroyActor)))))))
    (:CastFailed
      (if (!= OtherActor self)
        (goto _label)))))

(event EventBeginPlay
  (|CallParentFunction) ; This node is disabled and will not be called.\nDrag off pins to build functionality.
)

(event Collision|EventActorBeginOverlap
  (params (OtherActor :type Actor%20Object%20Reference))
  (|CallParentFunction OtherActor) ; This node is disabled and will not be called.\nDrag off pins to build functionality.
)

(event EventTick
  (params (DeltaSeconds :type Float%20%28single-precision%29))
  (|CallParentFunction DeltaSeconds))

(fn ConstructionScript
  (|CallParentFunction))