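; Rust bomb ability projectile that deals impact damage, then becomes a short-lived damage-over-time area.
; Hitting an opposing-type fighter or any non-fighter actor stops it, removes the hit sphere and starts a looping timer.
; Each tick damages opposing fighters in a second sphere, with all damage scaled by the owner ability's type attitudes.
; After a fixed tick count, or if the owner ability becomes invalid, a timeline shrinks it to destruction.
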(event OnComponentBeginOverlap(Sphere)
  (params (OverlappedComponent :type Primitive%20Component%20Object%20Reference) (OtherActor :type Actor%20Object%20Reference) (OtherComp :type Primitive%20Component%20Object%20Reference) (OtherBodyIndex :type Integer) (bFromSweep :type Boolean) (SweepResult :type Hit%20Result%20Structure%20%28by%20ref%29))
  (bind _asbp_fighter_character (Utilities|Casting|CastToBP_FighterCharacter OtherActor)
    (:then
      (if (Utilities|Enum|NotEqual(Enum) (Variables|/Game/Shota/Blueprints/Abilities/BP_Ability.BP_Ability_C|GetType (Variables|/Game/Shota/Blueprints/Fighter/BP_FighterCharacter.BP_FighterCharacter_C|GetAbility _asbp_fighter_character)) (Variables|/Game/Shota/Blueprints/Abilities/BP_Ability.BP_Ability_C|GetType (Variables|Default|GetOwnerAbility)))
        (Default|FApplyDamage _asbp_fighter_character (* (Variables|Default|GetDamage) (CallFunction|FLGetAttitude (Variables|/Game/Shota/Blueprints/Abilities/BP_Ability.BP_Ability_C|GetType (Variables|/Game/Shota/Blueprints/Fighter/BP_FighterCharacter.BP_FighterCharacter_C|GetAbility _asbp_fighter_character)) (Variables|/Game/Shota/Blueprints/Abilities/BP_Ability.BP_Ability_C|GetAttitudes (Variables|Default|GetOwnerAbility)))))
        (Default|CallOnHit :!label _label)
        (Utilities|FlowControl|DoOnce false
          (:Completed
            (Components|DestroyComponent (Variables|Default|GetSphere))
            (bind _returnvalue (Utilities|Time|SetTimerbyEvent (delegate Custom|OnPoisonUpdate) 0.5 true))
            (Variables|/Script/Engine.ProjectileMovementComponent|SetbSimulationEnabled (Variables|Default|GetProjectileMovement) false)))))
    (:CastFailed
      (if (!= OtherActor self)
        (goto _label)))))

(event Custom|OnPoisonUpdate
  (bind _result (Math|Integer|IncrementInt (Variables|Default|GetPoisonCount))
    (:%20%20
      (if (Utilities|IsValid (Variables|Default|GetOwnerAbility))
        (if (== _result 6)
          (Utilities|FlowControl|Sequence
            (:then_0
              (for _array_element (Collision|GetOverlappingActors (Variables|Default|GetSphere1) "/Game/Shota/Blueprints/Fighter/BP_FighterCharacter.BP_FighterCharacter_C" :!class /Script/Engine.PrimitiveComponent) :!label _label
                (bind _asbp_fighter_character (Utilities|Casting|CastToBP_FighterCharacter _array_element))
                (Utilities|IsValid (Variables|/Game/Shota/Blueprints/Fighter/BP_FighterCharacter.BP_FighterCharacter_C|GetAbility _asbp_fighter_character)
                  (:Is%20Valid
                    (if (Utilities|Enum|NotEqual(Enum) (Variables|/Game/Shota/Blueprints/Abilities/BP_Ability.BP_Ability_C|GetType (Variables|/Game/Shota/Blueprints/Fighter/BP_FighterCharacter.BP_FighterCharacter_C|GetAbility _asbp_fighter_character)) (Variables|/Game/Shota/Blueprints/Abilities/BP_Ability.BP_Ability_C|GetType (Variables|Default|GetOwnerAbility)))
                      (Default|FApplyDamage _asbp_fighter_character (* (Variables|Default|GetTickingDamage) (CallFunction|FLGetAttitude (Variables|/Game/Shota/Blueprints/Abilities/BP_Ability.BP_Ability_C|GetType (Variables|/Game/Shota/Blueprints/Fighter/BP_FighterCharacter.BP_FighterCharacter_C|GetAbility _asbp_fighter_character)) (Variables|/Game/Shota/Blueprints/Abilities/BP_Ability.BP_Ability_C|GetAttitudes (Variables|Default|GetOwnerAbility))))))))))
            (:then_1
              (bind _size (Timeline|ShrinkToDeath PlayFromStart)
                (:Update
                  (Transformation|SetActorScale3D (Math|Conversions|ToVector(Float) _size)))
                (:Finished
                  (Actor|DestroyActor)))))
          (else
            (goto _label)))
        (else
          (Utilities|Time|ClearandInvalidateTimerbyHandle (stale OnComponentBeginOverlap(Sphere) _returnvalue))
          (Timeline|ShrinkToDeath PlayFromStart))))))

(event EventBeginPlay
  (|CallParentFunction) ; This node is disabled and will not be called.\nDrag off pins to build functionality.
)

(event Collision|EventActorBeginOverlap
  (params (OtherActor :type Actor%20Object%20Reference))
  (|CallParentFunction OtherActor) ; This node is disabled and will not be called.\nDrag off pins to build functionality.
)

(event EventTick
  (params (DeltaSeconds :type Float%20%28single-precision%29))
  (|CallParentFunction DeltaSeconds))

(fn ConstructionScript
  (|CallParentFunction))