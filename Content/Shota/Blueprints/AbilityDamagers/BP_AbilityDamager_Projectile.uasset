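; BP_AbilityDamager_Projectile is a projectile ability damager that adds audiovisual feedback on hit.
; On BeginPlay it calls the parent, then binds a handler to the OnHit event.
; The handler plays a hit sound with basic attenuation and spawns a hit effect system at the actor's location.
; The Blueprint's own graphs contain no damage or movement logic.
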(event Custom|OnHitEvent
  (bind _returnvalue (Transformation|GetActorLocation))
  (Audio|PlaySoundatLocation (Variables|Default|GetHitSound) _returnvalue "0, 0, 0" 1.0 1.0 0.0 "/Game/Shota/Sounds/SA_Basic.SA_Basic" 0 0 0)
  (Niagara|SpawnSystematLocation (Variables|Default|GetHitEffect) _returnvalue))

(event EventBeginPlay
  (|CallParentFunction)
  (EventDispatchers|BindEventtoOnHit (delegate Custom|OnHitEvent)))

(event Collision|EventActorBeginOverlap
  (params (OtherActor :type Actor%20Object%20Reference))
  (|CallParentFunction OtherActor) ; This node is disabled and will not be called.\nDrag off pins to build functionality.
)

(event EventTick
  (params (DeltaSeconds :type Float%20%28single-precision%29))
  (|CallParentFunction DeltaSeconds) ; This node is disabled and will not be called.\nDrag off pins to build functionality.
)

(fn ConstructionScript
  (|CallParentFunction))