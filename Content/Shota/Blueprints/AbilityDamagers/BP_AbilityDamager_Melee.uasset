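; Melee ability damager actor that deals a single instant area hit to fighter characters, then destroys itself.
; On BeginPlay it waits one tick, then gathers every BP_FighterCharacter overlapping its Sphere.
; Fighters whose ability type differs from the owner's take Damage scaled by the owner's attitude multiplier toward their type, looked up through FLGetAttitude.
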(event EventBeginPlay
  (|CallParentFunction)
  (Utilities|FlowControl|DelayUntilNextTick)
  (for _array_element (Collision|GetOverlappingActors (Variables|Default|GetSphere) "/Game/Shota/Blueprints/Fighter/BP_FighterCharacter.BP_FighterCharacter_C" :!class /Script/Engine.PrimitiveComponent)
    (bind _asbp_fighter_character (Utilities|Casting|CastToBP_FighterCharacter _array_element))
    (if (Utilities|Enum|NotEqual(Enum) (Variables|/Game/Shota/Blueprints/Abilities/BP_Ability.BP_Ability_C|GetType (Variables|/Game/Shota/Blueprints/Fighter/BP_FighterCharacter.BP_FighterCharacter_C|GetAbility _asbp_fighter_character)) (Variables|/Game/Shota/Blueprints/Abilities/BP_Ability.BP_Ability_C|GetType (Variables|Default|GetOwnerAbility)))
      (Default|FApplyDamage _asbp_fighter_character (* (Variables|Default|GetDamage) (CallFunction|FLGetAttitude (Variables|/Game/Shota/Blueprints/Abilities/BP_Ability.BP_Ability_C|GetType (Variables|/Game/Shota/Blueprints/Fighter/BP_FighterCharacter.BP_FighterCharacter_C|GetAbility _asbp_fighter_character)) (Variables|/Game/Shota/Blueprints/Abilities/BP_Ability.BP_Ability_C|GetAttitudes (Variables|Default|GetOwnerAbility)))))))
  (Actor|DestroyActor))

(event Collision|EventActorBeginOverlap
  (params (OtherActor :type Actor%20Object%20Reference))
  (|CallParentFunction OtherActor) ; This node is disabled and will not be called.\nDrag off pins to build functionality.
)

(event EventTick
  (params (DeltaSeconds :type Float%20%28single-precision%29))
  (|CallParentFunction DeltaSeconds) ; This node is disabled and will not be called.\nDrag off pins to build functionality.
)

(fn ConstructionScript
  (|CallParentFunction))