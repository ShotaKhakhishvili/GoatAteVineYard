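; Ability damager for the gun bomb, which deals area damage to fighter characters when triggered.
; An overlap on the Sphere component triggers it, and Sphere1 gathers every BP_FighterCharacter inside as a damage target.
; While the owner ability is valid, each target takes Damage scaled by the attitude of that ability toward the target's ability type.
; It then fires OnHit and destroys itself.
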(event OnComponentBeginOverlap(Sphere)
  (params (OverlappedComponent :type Primitive%20Component%20Object%20Reference) (OtherActor :type Actor%20Object%20Reference) (OtherComp :type Primitive%20Component%20Object%20Reference) (OtherBodyIndex :type Integer) (bFromSweep :type Boolean) (SweepResult :type Hit%20Result%20Structure%20%28by%20ref%29))
  (for _array_element (Collision|GetOverlappingActors (Variables|Default|GetSphere1) "/Game/Shota/Blueprints/Fighter/BP_FighterCharacter.BP_FighterCharacter_C" :!class /Script/Engine.PrimitiveComponent)
    (Utilities|IsValid (Variables|Default|GetOwnerAbility)
      (:Is%20Valid
        (bind _asbp_fighter_character (Utilities|Casting|CastToBP_FighterCharacter _array_element))
        (Default|FApplyDamage _asbp_fighter_character (* (Variables|Default|GetDamage) (CallFunction|FLGetAttitude (Variables|/Game/Shota/Blueprints/Abilities/BP_Ability.BP_Ability_C|GetType (Variables|/Game/Shota/Blueprints/Fighter/BP_FighterCharacter.BP_FighterCharacter_C|GetAbility _asbp_fighter_character)) (Variables|/Game/Shota/Blueprints/Abilities/BP_Ability.BP_Ability_C|GetAttitudes (Variables|Default|GetOwnerAbility))))))))
  (Default|CallOnHit)
  (Actor|DestroyActor))

(fn ConstructionScript
  (|CallParentFunction))