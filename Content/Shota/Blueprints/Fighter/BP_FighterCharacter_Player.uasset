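; Player-controlled fighter that collects droppables to fill a meter, then transforms into that type to gain its ability.
; A full meter lets T spawn and swap the Ability actor, then advance DroppableType along a fixed chain, resetting count and updating followers and the WBP_Game HUD.
; E and Q drive abilities, C skips to the next type, and death hides the character.
; Tick skips the parent's bot rotation logic.
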(event Custom|EventOnPlayerDead
  ;[0.15 0.15 0.15 0.5] CHANGEEE
  (CallFunction|Died)
  (Variables|Default|SetDied_0 true)
  (Variables|Default|SetHP 9999999999.0)
  (Rendering|SetVisibility (Variables|Character|GetMesh) false false)
  (Collision|SetCollisionEnabled (Variables|Default|GetCapsuleComponent) "NoCollision")
  (Pawn|Components|CharacterMovement|SetMovementMode (Variables|Character|GetCharacterMovement) "MOVE_None" 0))

(event Custom|ChangeMaskingSearch
  ;[0.15 0.15 0.15 0.5] Changing What You Want To Mask Into?
  (CallFunction|FSetNextDroppable)
  (CallFunction|ResetFollowingBoyos)
  (Default|CallDroppableReceived))

(event Custom|EventOnDroppable
  (Audio|PlaySoundatLocation "/Game/Gigi/Audio/Sounds/UI_elements/BubblePop/ES_Ascending_x4_-_Epidemic_Sound_001.ES_Ascending_x4_-_Epidemic_Sound_001" (Transformation|GetActorLocation) "0, 0, 0" 0.6 1.0 0.0 "/Game/Shota/Sounds/SA_Basic.SA_Basic" 0 0 0)
  (bind _result (Math|Integer|IncrementInt (Variables|Default|GetDroppableCount))
    (:%20%20
      (if (>= _result (Variables|Default|GetDroppableMaxCount))
        (Default|CallDroppablesFilled)
        (Variables|Default|SetCanTransform true)))))

(event Custom|Transform
  (Niagara|SpawnSystematLocation "/Game/NiagaraExamples/FX_Explosions/NS_Dirt_Explosion.NS_Dirt_Explosion" (Transformation|GetActorLocation))
  (Audio|PlaySoundatLocation "/Game/Shota/Sounds/Explosion4.Explosion4" (Transformation|GetActorLocation) "0, 0, 0" 1.5 1.0 0.0 "/Game/Shota/Sounds/SA_Basic.SA_Basic" 0 0 0)
  (Utilities|FlowControl|Delay 0.19)
  (bind _returnvalue (Game|SpawnActorfromClass (CallFunction|FLTypetoClass (Variables|Default|GetDroppableType)) (Math|Transform|MakeTransform "0, 0, 0" "0, 0, 0" "1.000000,1.000000,1.000000") "Undefined" "MultiplyWithRoot" 0 self 0))
  (Actor|DestroyActor (Variables|Default|GetAbility))
  (Variables|Default|SetAbility _returnvalue)
  (switch Utilities|FlowControl|Switch|SwitchonE_ThingType (Variables|Default|GetDroppableType)))

(event EventTick
  (params (DeltaSeconds :type Float%20%28single-precision%29))
  ;[0.15 0.15 0.15 0.5] Do not call parent tick, some bot movement rotation is written there
)

(event EventBeginPlay
  (|CallParentFunction)
  (EventDispatchers|BindEventtoDroppableReceived (delegate Custom|EventOnDroppable))
  (bind _returnvalue (UserInterface|CreateWidget "/Game/Shota/Widgets/WBP_Game.WBP_Game_C" 0 self))
  (bind _output_get (Variables|Default|SetWBP_Game _returnvalue))
  (UserInterface|Viewport|AddtoViewport _output_get 0)
  (EventDispatchers|BindEventtoOnDied (delegate Custom|EventOnPlayerDead)))

(event EventFPlayNext
  (params (FadeInSpeed :type Float%20%28double-precision%29) (Sound :type Sound%20Base%20Object%20Reference))
  (Default|PlayNext (Variables|Default|GetAC_Audio) FadeInSpeed Sound))

(event Input|KeyboardEvents|Q
  (params (Key :type Key%20Structure :default "None"))
  (:Pressed
    (Utilities|FNotDead
      (:NotDead
        (Default|ActivateSimpleAbility (Variables|Default|GetAbility)))))
  (:Released
    (Default|DeactivateSimpleAbility (Variables|Default|GetAbility))))

(event Input|KeyboardEvents|X
  (params (Key :type Key%20Structure :default "None"))
  (:Pressed
    (Utilities|FNotDead
      (:NotDead
        (Default|CallOnPauseButton)))))

(event Input|KeyboardEvents|E
  (params (Key :type Key%20Structure :default "None"))
  (:Pressed
    (Utilities|FNotDead
      (:NotDead
        (Default|ActivateAbility (Variables|Default|GetAbility))))))

(event Input|KeyboardEvents|T
  (params (Key :type Key%20Structure :default "None"))
  (bind _ability (Variables|Default|GetAbility))
  (:Pressed
    (Utilities|FNotDead
      (:NotDead
        (if (Variables|Default|GetCanTransform)
          (Variables|Default|SetCanTransform false)
          (CallFunction|Transform)
          (Utilities|FlowControl|Delay 0.2)
          (CallFunction|ChangeMaskingSearch)
          (Default|Update (Variables|/Game/Shota/Widgets/WBP_Game.WBP_Game_C|GetWBP_Mask (Variables|Default|GetWBP_Game)) (Variables|/Game/Shota/Blueprints/Abilities/BP_Ability.BP_Ability_C|GetMasks (Variables|Default|GetAbility)))
          (Variables|/Game/Shota/Blueprints/Abilities/BP_Ability.BP_Ability_C|SetDamageMultiplier _ability 1.0)
          (Variables|/Game/Shota/Blueprints/Abilities/BP_Ability.BP_Ability_C|SetSpeedMultiplier _ability 1.0)
          (Variables|/Script/Engine.CharacterMovementComponent|SetMaxWalkSpeed (Variables|Character|GetCharacterMovement) 5e+02)
          (Default|RefreshAbilityIcons (Variables|Default|GetWBP_Game)))))))

(event Input|KeyboardEvents|C
  (params (Key :type Key%20Structure :default "None"))
  ;[0.15 0.15 0.15 0.5] Changing What You Want To Mask Into?
  (:Pressed
    (CallFunction|ChangeMaskingSearch)))

(fn ConstructionScript
  (|CallParentFunction))

(fn FSetNextDroppable
  (Variables|Default|SetDroppableCount 0)
  (switch Utilities|FlowControl|Switch|SwitchonE_ThingType (Variables|Default|GetDroppableType)
    (:NewEnumerator1
      (Variables|Default|SetDroppableType "NewEnumerator0")
      (Variables|Default|SetDroppableMaxCount 1)
      (Variables|Default|SetDroppableText "ვენახომეტრი???"))
    (:NewEnumerator2
      (Variables|Default|SetDroppableType "NewEnumerator1")
      (Variables|Default|SetDroppableMaxCount 5)
      (Variables|Default|SetDroppableText "თხებომეტრი"))
    (:NewEnumerator3
      (Variables|Default|SetDroppableType "NewEnumerator2")
      (Variables|Default|SetDroppableMaxCount 5)
      (Variables|Default|SetDroppableText "მგელომეტრი"))
    (:NewEnumerator4
      (Variables|Default|SetDroppableType "NewEnumerator3")
      (Variables|Default|SetDroppableMaxCount 4)
      (Variables|Default|SetDroppableText "თოფომეტრი"))
    (:NewEnumerator5
      (Variables|Default|SetDroppableType "NewEnumerator4")
      (Variables|Default|SetDroppableMaxCount 5)
      (Variables|Default|SetDroppableText "ჟანგომეტრი"))
    (:NewEnumerator6
      (Variables|Default|SetDroppableType "NewEnumerator5")
      (Variables|Default|SetDroppableMaxCount 4)
      (Variables|Default|SetDroppableText "მიწომეტრი"))
    (:NewEnumerator7
      (Variables|Default|SetDroppableType "NewEnumerator6")
      (Variables|Default|SetDroppableMaxCount 5)
      (Variables|Default|SetDroppableText "თაგვომეტრი"))))

(fn ResetFollowingBoyos
  (for _array_element (Variables|Default|GetDropableItems)
    (LocalVariables|SetLastBoyo _array_element)
    (Utilities|IsValid (LocalVariables|GetLastBoyo)
      (:Is%20Valid
        (Utilities|Array|Add (LocalVariables|GetFollowingBoyos) (LocalVariables|GetLastBoyo))
        (Class|CharacterTransformed|Transformed(Message) (LocalVariables|GetLastBoyo) (Variables|Default|GetDroppableType)))))
  (LocalVariables|SetFollowingBoyos (LocalVariables|GetFollowingBoyos))
  (return))