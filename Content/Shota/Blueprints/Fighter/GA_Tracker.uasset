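; GA_Tracker is a Blueprint that tracks a count of goats and reacts when none remain.
; Decreasegoat decrements the count, prints it as debug text and, at zero or below, sets a Figures flag.
; It then finds the BP_FighterCharacter_Player by class and calls Didnteat on that player's game widget.
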(fn Decreasegoat
  (bind _output_get (Variables|Default|Setgoats (- (Variables|Default|Getgoats) 1)))
  (Development|PrintString (Utilities|String|Append "asdas" (Utilities|String|ToString(Integer) _output_get)))
  (if (<= _output_get 0)
    (bind _returnvalue (Actor|GetActorOfClass "/Game/Shota/Blueprints/Fighter/BP_FighterCharacter_Player.BP_FighterCharacter_Player_C"))
    (Variables|Default|Setfigures true)
    (Default|Didnteat (Variables|/Game/Shota/Blueprints/Fighter/BP_FighterCharacter_Player.BP_FighterCharacter_Player_C|GetWBP_Game _returnvalue))))