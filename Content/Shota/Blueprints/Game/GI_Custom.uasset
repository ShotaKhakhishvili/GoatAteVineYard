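; Custom Game Instance that manages the player's saved options: audio volumes, mouse sensitivity, cursor and landscape quality.
; FInitialize loads the SG_Default save from the options slot, or creates and saves a new one.
; Per-setting save events only edit the cached SOptions struct, load functions read from it, and FApplySaves writes it to disk.
; Finished separately flags the game as finished and calls Didnteat on the fighter player's game widget.
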(event EventFSaveLandscapeQuality
  (params (LandcapeQuality :type Integer))
  (Utilities|Struct|SetmembersinS_Options (Variables|/Game/Shota/Blueprints/Game/SG_Default.SG_Default_C|GetS_Options (Variables|Default|GetSG_Default)) LandcapeQuality))

(event EventFSaveCursorID
  (params (CursorID :type Integer))
  (Utilities|Struct|SetmembersinS_Options (Variables|/Game/Shota/Blueprints/Game/SG_Default.SG_Default_C|GetS_Options (Variables|Default|GetSG_Default)) CursorID))

(event EventFSaveSFXVolume
  (params (Volume :type Float%20%28double-precision%29))
  (Utilities|Struct|SetmembersinS_Options (Variables|/Game/Shota/Blueprints/Game/SG_Default.SG_Default_C|GetS_Options (Variables|Default|GetSG_Default)) Volume))

(event EventFInitialize
  (bind _returnvalue (SaveGame|DoesSaveGameExist (Variables|Default|GetOptionsSaveName)))
  (if _returnvalue
    (bind _returnvalue_2 (SaveGame|LoadGamefromSlot (Variables|Default|GetOptionsSaveName)))
    (bind _assg_default (Utilities|Casting|CastToSG_Default _returnvalue_2))
    (Variables|Default|SetSG_Default _assg_default)
    (else
      (bind _returnvalue_3 (SaveGame|CreateSaveGameObject "/Game/Shota/Blueprints/Game/SG_Default.SG_Default_C"))
      (bind _output_get (Variables|Default|SetSG_Default _returnvalue_3))
      (SaveGame|SaveGametoSlot _output_get (Variables|Default|GetOptionsSaveName)))))

(event EventFSaveMouseSensitivity
  (params (Sensitivity :type Float%20%28double-precision%29))
  (Utilities|Struct|SetmembersinS_Options (Variables|/Game/Shota/Blueprints/Game/SG_Default.SG_Default_C|GetS_Options (Variables|Default|GetSG_Default)) Sensitivity))

(event EventFSaveMusicVolume
  (params (Volume :type Float%20%28double-precision%29))
  (Utilities|Struct|SetmembersinS_Options (Variables|/Game/Shota/Blueprints/Game/SG_Default.SG_Default_C|GetS_Options (Variables|Default|GetSG_Default)) Volume))

(event EventFSaveUIVolume
  (params (Volume :type Float%20%28double-precision%29))
  (Utilities|Struct|SetmembersinS_Options (Variables|/Game/Shota/Blueprints/Game/SG_Default.SG_Default_C|GetS_Options (Variables|Default|GetSG_Default)) Volume))

(event EventFSaveMasterVolume
  (params (Volume :type Float%20%28double-precision%29))
  (Utilities|Struct|SetmembersinS_Options (Variables|/Game/Shota/Blueprints/Game/SG_Default.SG_Default_C|GetS_Options (Variables|Default|GetSG_Default)) Volume))

(fn Finished
  (bind _returnvalue (Actor|GetActorOfClass "/Game/Shota/Blueprints/Fighter/BP_FighterCharacter_Player.BP_FighterCharacter_Player_C"))
  (Variables|Default|SetFinishedGame true)
  (Default|Didnteat (Variables|/Game/Shota/Blueprints/Fighter/BP_FighterCharacter_Player.BP_FighterCharacter_Player_C|GetWBP_Game _returnvalue)))

(fn FApplySaves
  (bind _returnvalue (SaveGame|SaveGametoSlot (Variables|Default|GetSG_Default) (Variables|Default|GetOptionsSaveName)))
  (return _returnvalue))

(fn FLoadCursorID
  (return (.O_Cursor (Utilities|Struct|BreakS_Options (Variables|/Game/Shota/Blueprints/Game/SG_Default.SG_Default_C|GetS_Options (Variables|Default|GetSG_Default))))))

(fn FLoadLandscapeQuality
  (return (.G_Landscape (Utilities|Struct|BreakS_Options (Variables|/Game/Shota/Blueprints/Game/SG_Default.SG_Default_C|GetS_Options (Variables|Default|GetSG_Default))))))

(fn FLoadMasterVolume
  (return (.M_Master (Utilities|Struct|BreakS_Options (Variables|/Game/Shota/Blueprints/Game/SG_Default.SG_Default_C|GetS_Options (Variables|Default|GetSG_Default))))))

(fn FLoadMouseSensitivity
  (return (.O_Mouse (Utilities|Struct|BreakS_Options (Variables|/Game/Shota/Blueprints/Game/SG_Default.SG_Default_C|GetS_Options (Variables|Default|GetSG_Default))))))

(fn FLoadMusicVolume
  (return (.M_Music (Utilities|Struct|BreakS_Options (Variables|/Game/Shota/Blueprints/Game/SG_Default.SG_Default_C|GetS_Options (Variables|Default|GetSG_Default))))))

(fn FLoadSFXVolume
  (return (.M_SFX (Utilities|Struct|BreakS_Options (Variables|/Game/Shota/Blueprints/Game/SG_Default.SG_Default_C|GetS_Options (Variables|Default|GetSG_Default))))))

(fn FLoadUIVolume
  (return (.M_UI (Utilities|Struct|BreakS_Options (Variables|/Game/Shota/Blueprints/Game/SG_Default.SG_Default_C|GetS_Options (Variables|Default|GetSG_Default))))))