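; BP_Ability_Rat is a character ability that gives its owner a speed boost and a lunging melee attack, and sets the owner's anim class on BeginPlay.
; The cooldown-gated main ability raises walk speed, loops random footstep sounds for about five seconds via a delayed counter that is never reset, then lowers speed.
; The simple ability, gated by cooldown and falling checks, launches the character, plays a punch montage and spawns a melee damager ahead.
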(event EventActivateSimpleAbility
  (bind _owneractor (Variables|Default|GetOwnerActor))
  (bind _returnvalue (Transformation|GetActorTransform _owneractor))
  (if (not (CallFunction|FHasCooldownorFallingS))
    (|CallParentFunction)
    (Audio|PlaySoundatLocation "/Game/Shota/Sounds/Jumps/CatJumpLand.CatJumpLand" (Transformation|GetActorLocation (Variables|Default|GetOwnerActor)) "0, 0, 0" 1.0 1.0 0.0 "/Game/Gigi/Audio/AbilityCat.AbilityCat" 0 0 0)
    (CallFunction|FLaunchCharacter 5e+02 5e+01)
    (Animation|Montage|PlayMontage (Variables|/Script/Engine.Character|GetMesh (Variables|Default|GetOwnerActor)) "/Game/Shota/Assets/Things/Cat/NewOnes/AM_CatPunch.AM_CatPunch"
      (:then
        (Utilities|FlowControl|Delay 0.2)
        (Game|SpawnActorfromClass "/Game/Shota/Blueprints/AbilityDamagers/BP_AbilityDamager_Melee.BP_AbilityDamager_Melee_C" (Math|Transform|MakeTransform (+ (.location _returnvalue) "0.000000,0.000000,50.000000" (* (Transformation|GetActorForwardVector _owneractor) 5e+01)) (.rotation _returnvalue) (.scale _returnvalue)) "Undefined" "MultiplyWithRoot" 0 self 0 0)))))

(event EventBeginPlay
  (|CallParentFunction)
  (Components|SkeletalMesh|SetAnimInstanceClass (Variables|/Script/Engine.Character|GetMesh (Variables|Default|GetOwnerActor)) "/Game/Shota/Blueprints/Fighter/ABPS/ABP_Wruwuna.ABP_Wruwuna_C"))

(event EventActivateAbility
  (bind _owneractor (Variables|Default|GetOwnerActor))
  (bind _charactermovement (Variables|/Script/Engine.Character|GetCharacterMovement _owneractor))
  (if (not (CallFunction|FHasCooldown))
    (|CallParentFunction)
    (Variables|/Script/Engine.CharacterMovementComponent|SetMaxWalkSpeed _charactermovement 1e+03)
    (Audio|PlaySoundatLocation (.OutItem (Utilities|Array|Random (Utilities|Array|MakeArray "/Game/Gigi/Audio/Sounds/Footsteps/Soft_Step_Variations/Soft_Step2.Soft_Step2" "/Game/Shota/Sounds/Footsteps/Soft_Step_Variations/Soft_Step5.Soft_Step5" "/Game/Gigi/Audio/Sounds/Footsteps/Soft_Step_Variations/Soft_Step5.Soft_Step5" "/Game/Shota/Sounds/Footsteps/Soft_Step_Variations/Soft_Step4.Soft_Step4" "/Game/Gigi/Audio/Sounds/Footsteps/Soft_Step_Variations/Soft_Step4.Soft_Step4" "/Game/Shota/Sounds/Footsteps/Soft_Step_Variations/Soft_Step3.Soft_Step3" "/Game/Gigi/Audio/Sounds/Footsteps/Soft_Step_Variations/Soft_Step3.Soft_Step3" "/Game/Shota/Sounds/Footsteps/Soft_Step_Variations/Soft_Step2.Soft_Step2"))) (Transformation|GetActorLocation (Variables|Default|GetOwnerActor)) "0, 0, 0" 1.0 1.0 0.0 "/Game/Gigi/Audio/AbilityCat.AbilityCat" 0 0 0 :!label _label)
    (Math|Float|IncrementFloat (Variables|Default|Getn)
      (:%20%20
        (Utilities|FlowControl|Delay 0.2)
        (if (== (Variables|Default|Getn) 25.0)
          (Variables|/Script/Engine.CharacterMovementComponent|SetMaxWalkSpeed _charactermovement 5e+02)
          (else
            (goto _label)))))))

(fn ConstructionScript
  (|CallParentFunction))