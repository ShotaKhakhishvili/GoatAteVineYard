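; BP_Ability is an ability Blueprint that gives its owner actor a simple ability and a main one, each with its own cooldown.
; On BeginPlay it swaps the owner's skeletal mesh.
; Each activation event plays a montage on that mesh and immediately resets its timer, without checking it first.
; Tick counts both timers down, and two functions report whether each is still cooling down.
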(event Custom|ActivateAbility
  (Animation|Montage|PlayMontage (Variables|/Script/Engine.Character|GetMesh (Variables|Default|GetOwnerActor)) 0
    (:then
      (Variables|Default|SetCooldown (Variables|Default|GetMaxCooldown)))))

(event Custom|ActivateSimpleAbility
  (Animation|Montage|PlayMontage (Variables|/Script/Engine.Character|GetMesh (Variables|Default|GetOwnerActor)) 0
    (:then
      (Variables|Default|SetCooldown_S (Variables|Default|GetMaxCooldown_S)))))

(event EventTick
  (params (DeltaSeconds :type Float%20%28single-precision%29))
  (Variables|Default|SetCooldown (- (Variables|Default|GetCooldown) DeltaSeconds))
  (Variables|Default|SetCooldown_S (- (Variables|Default|GetCooldown_S) DeltaSeconds)))

(event EventBeginPlay
  (Components|SkeletalMesh|SetSkeletalMeshAsset (Variables|/Script/Engine.Character|GetMesh (Variables|Default|GetOwnerActor)) (Variables|Default|GetSkeletalMesh)))

(fn ConstructionScript)

(fn FHasCooldown
  (return (>= (Variables|Default|GetCooldown) 0.0)))

(fn FHasCooldownS
  (return (>= (Variables|Default|GetCooldown_S) 0.0)))