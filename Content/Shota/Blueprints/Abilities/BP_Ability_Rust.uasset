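; Rust ability for a character, with a main bomb attack and a simple bullet attack.
; On BeginPlay it switches the owner's mesh to the Rust animation Blueprint.
; Each attack passes its cooldown check (the simple one also checks falling), launches the character with negative strength, then plays a throw montage and wind sound.
; After a short delay synced to the throw, it spawns its damager above the owner, passing itself as OwnerAbility.
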(event EventActivateSimpleAbility
  (bind _owneractor (Variables|Default|GetOwnerActor))
  (bind _returnvalue (Transformation|GetActorTransform _owneractor))
  (if (not (CallFunction|FHasCooldownorFallingS))
    (|CallParentFunction)
    (CallFunction|FLaunchCharacter -7.5e+02 5e+01)
    (Animation|Montage|PlayMontage (Variables|/Script/Engine.Character|GetMesh (Variables|Default|GetOwnerActor)) "/Game/Shota/Assets/Things/Rust/AM_RustThrow.AM_RustThrow"
      (:then
        (Audio|PlaySoundatLocation "/Game/Gigi/Audio/Sounds/Jumps/WindyJumps/ES_Organic__Wind__Cool__Fast_-_Epidemic_Sound_003.ES_Organic__Wind__Cool__Fast_-_Epidemic_Sound_003" (Transformation|GetActorLocation (Variables|Default|GetOwnerActor)) "0, 0, 0" 1.0 1.0 0.0 "/Game/Gigi/Audio/AbilityCat.AbilityCat" 0 0 0)
        (Utilities|FlowControl|Delay 0.55)
        (Game|SpawnActorfromClass "/Game/Shota/Blueprints/AbilityDamagers/BP_AbilityDamager_RustBullet.BP_AbilityDamager_RustBullet_C" (Math|Transform|MakeTransform (+ (.location _returnvalue) "0.000000,0.000000,100.000000") (.rotation _returnvalue) (.scale _returnvalue)) "Undefined" "MultiplyWithRoot" 0 self 0)))))

(event EventBeginPlay
  (|CallParentFunction)
  (Components|SkeletalMesh|SetAnimInstanceClass (Variables|/Script/Engine.Character|GetMesh (Variables|Default|GetOwnerActor)) "/Game/Shota/Blueprints/Fighter/ABPS/ABP_Rust.ABP_Rust_C"))

(event EventActivateAbility
  (bind _owneractor (Variables|Default|GetOwnerActor))
  (bind _returnvalue (Transformation|GetActorTransform _owneractor))
  (if (not (CallFunction|FHasCooldown))
    (|CallParentFunction)
    (CallFunction|FLaunchCharacter -1e+03 5e+01)
    (Animation|Montage|PlayMontage (Variables|/Script/Engine.Character|GetMesh (Variables|Default|GetOwnerActor)) "/Game/Shota/Assets/Things/Rust/AM_RustThrow.AM_RustThrow"
      (:then
        (Audio|PlaySoundatLocation "/Game/Shota/Sounds/Jumps/WindyJumps/ES_Organic__Wind__Cool__Fast_-_Epidemic_Sound_001.ES_Organic__Wind__Cool__Fast_-_Epidemic_Sound_001" (Transformation|GetActorLocation (Variables|Default|GetOwnerActor)) "0, 0, 0" 1.0 1.0 0.0 "/Game/Gigi/Audio/AbilityCat.AbilityCat" 0 0 0)
        (Utilities|FlowControl|Delay 0.55)
        (Game|SpawnActorfromClass "/Game/Shota/Blueprints/AbilityDamagers/BP_AbilityDamager_RustBomb.BP_AbilityDamager_RustBomb_C" (Math|Transform|MakeTransform (+ (.location _returnvalue) "0.000000,0.000000,100.000000") (.rotation _returnvalue) (.scale _returnvalue)) "Undefined" "MultiplyWithRoot" 0 self 0)))))

(fn ConstructionScript
  (|CallParentFunction))