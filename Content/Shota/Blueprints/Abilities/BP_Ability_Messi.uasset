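; Messi character ability that applies the Messi anim blueprint to its owner on BeginPlay and provides a main and a simple attack, both cooldown-gated.
; The main ability spawns a GoatRock damager at the mesh's "Poop" socket.
; The simple ability, also blocked while falling, launches the character and plays a bite montage, spawning an actor with hit sounds at the melee socket after a short delay.
; Montage completion restores walking movement.
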(event EventActivateSimpleAbility
  (if (not (CallFunction|FHasCooldownorFallingS))
    (|CallParentFunction)
    (CallFunction|FLaunchCharacter 7.5e+02 5e+01)
    (Animation|Montage|PlayMontage (Variables|/Script/Engine.Character|GetMesh (Variables|Default|GetOwnerActor)) "/Game/Gigi/NewCharacters/Messi/Messi_bite_Montage.Messi_bite_Montage"
      (:then
        (Utilities|FlowControl|Delay 0.3)
        (Game|SpawnActorfromClass "/Game/Shota/Blueprints/AbilityDamagers/BP_AbilityDamager_Melee.BP_AbilityDamager_Melee_C" (Transformation|GetSocketTransform (Variables|/Script/Engine.Character|GetMesh (Variables|Default|GetOwnerActor)) "MeleeSocket" "RTS_World") "Undefined" "MultiplyWithRoot" 0 self (Variables|Default|GetSimpleAbilityHitSounds) 0))
      (:OnCompleted
        (Pawn|Components|CharacterMovement|SetMovementMode (Variables|/Script/Engine.Character|GetCharacterMovement (Variables|Default|GetOwnerActor)) "MOVE_Walking" 0)))))

(event EventBeginPlay
  (|CallParentFunction)
  (Components|SkeletalMesh|SetAnimInstanceClass (Variables|/Script/Engine.Character|GetMesh (Variables|Default|GetOwnerActor)) "/Game/Gigi/NewCharacters/ABPS/ABP_Messi.ABP_Messi_C"))

(event EventActivateAbility
  (if (not (CallFunction|FHasCooldown))
    (Game|SpawnActorfromClass "/Game/Shota/Blueprints/AbilityDamagers/BP_AbilityDamager_GoatRock.BP_AbilityDamager_GoatRock_C" (Transformation|GetSocketTransform (Variables|/Script/Engine.Character|GetMesh (Variables|Default|GetOwnerActor)) "Poop" "RTS_World") "Undefined" "MultiplyWithRoot" 0 self 0 0)
    (|CallParentFunction)))

(fn ConstructionScript
  (|CallParentFunction))