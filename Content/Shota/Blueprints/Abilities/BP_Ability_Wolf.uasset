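; Wolf ability set that applies the wolf animation class to its owner and provides two cooldown-gated abilities.
; The main ability plays a howl montage and doubles damage temporarily, restoring walking both as the montage starts and when it completes.
; The simple ability, also gated on falling, launches the character with a punch montage and sound, then spawns a melee damager in front after a short delay.
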(event EventActivateSimpleAbility
  (bind _owneractor (Variables|Default|GetOwnerActor))
  (bind _returnvalue (Transformation|GetActorTransform _owneractor))
  (if (not (CallFunction|FHasCooldownorFallingS))
    (|CallParentFunction)
    (CallFunction|FLaunchCharacter 6e+02 5e+01)
    (Animation|Montage|PlayMontage (Variables|/Script/Engine.Character|GetMesh (Variables|Default|GetOwnerActor)) "/Game/Shota/Assets/Things/Wolf/AM_WolfPunch.AM_WolfPunch"
      (:then
        (Audio|PlaySoundatLocation "/Game/Shota/Sounds/Jumps/CatJumpLand.CatJumpLand" (Transformation|GetActorLocation (Variables|Default|GetOwnerActor)) "0, 0, 0" 1.0 1.0 0.0 "/Game/Gigi/Audio/AbilityCat.AbilityCat" 0 0 0)
        (Utilities|FlowControl|Delay 0.5)
        (Game|SpawnActorfromClass "/Game/Shota/Blueprints/AbilityDamagers/BP_AbilityDamager_Melee.BP_AbilityDamager_Melee_C" (Math|Transform|MakeTransform (+ (.location _returnvalue) "0.000000,0.000000,50.000000" (* (Transformation|GetActorForwardVector _owneractor) 5e+01)) (.rotation _returnvalue) (.scale _returnvalue)) "Undefined" "MultiplyWithRoot" 0 self 0 0)))))

(event EventBeginPlay
  (|CallParentFunction)
  (Components|SkeletalMesh|SetAnimInstanceClass (Variables|/Script/Engine.Character|GetMesh (Variables|Default|GetOwnerActor)) "/Game/Shota/Blueprints/Fighter/ABPS/ABP_Wolf.ABP_Wolf_C"))

(event EventActivateAbility
  (if (not (CallFunction|FHasCooldown))
    (|CallParentFunction)
    (Variables|Default|SetDamageMultiplier 2.0)
    (Pawn|Components|CharacterMovement|SetMovementMode (Variables|/Script/Engine.Character|GetCharacterMovement (Variables|Default|GetOwnerActor)) "MOVE_None" 0)
    (Animation|Montage|PlayMontage (Variables|/Script/Engine.Character|GetMesh (Variables|Default|GetOwnerActor)) "/Game/Shota/Assets/Things/Wolf/AM_Howl.AM_Howl"
      (:then
        _)
      (:OnCompleted
        _))
    (Pawn|Components|CharacterMovement|SetMovementMode (Variables|/Script/Engine.Character|GetCharacterMovement (Variables|Default|GetOwnerActor)) "MOVE_Walking" 0)
    (Utilities|FlowControl|Delay 5.0)
    (Variables|Default|SetDamageMultiplier 1.0)))

(fn ConstructionScript
  (|CallParentFunction))