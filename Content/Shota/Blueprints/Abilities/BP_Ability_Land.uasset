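; Land (earth) ability that raises a rock in front of its owner, with a melee damager as the simple attack and the ABP_Mud anim class set on BeginPlay.
; The main ability requires a sphere-trace hit below the point ahead, then spawns a Nanite rock mesh below the owner's height.
; A looping timer steps the rock upward while owner movement is disabled.
; After a delay, the DieOut timeline drives its scale and destroys it.
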(event Custom|MoveUpStep
  (Transformation|AddActorWorldOffset (stale EventActivateAbility _returnvalue_6) "0.000000,0.000000,4.000000")
  (bind _result (Math|Integer|IncrementInt (Variables|Default|GetStepCount))
    (:%20%20
      (if (> _result 25)
        (Utilities|Time|ClearandInvalidateTimerbyHandle (stale EventActivateAbility _returnvalue_7))
        (Pawn|Components|CharacterMovement|SetMovementMode (Variables|/Script/Engine.Character|GetCharacterMovement (Variables|Default|GetOwnerActor)) "MOVE_Walking" 0)))))

(event EventActivateSimpleAbility
  (bind _owneractor (Variables|Default|GetOwnerActor))
  (bind _returnvalue (Transformation|GetActorTransform _owneractor))
  (if (not (CallFunction|FHasCooldownorFallingS))
    (Game|SpawnActorfromClass "/Game/Shota/Blueprints/AbilityDamagers/BP_AbilityDamager_Melee.BP_AbilityDamager_Melee_C" (Math|Transform|MakeTransform (+ (.location _returnvalue) "0.000000,0.000000,50.000000" (* (Transformation|GetActorForwardVector _owneractor) 5e+01)) (.rotation _returnvalue) (.scale _returnvalue)) "Undefined" "MultiplyWithRoot" 0 self 0)
    (|CallParentFunction)))

(event EventBeginPlay
  (|CallParentFunction)
  (Components|SkeletalMesh|SetAnimInstanceClass (Variables|/Script/Engine.Character|GetMesh (Variables|Default|GetOwnerActor)) "/Game/Shota/Blueprints/Fighter/ABPS/ABP_Mud.ABP_Mud_C"))

(event EventActivateAbility
  (bind _owneractor (Variables|Default|GetOwnerActor))
  (bind _owneractor_2 (Variables|Default|GetOwnerActor))
  (bind _returnvalue (Transformation|GetActorLocation _owneractor_2))
  (bind _returnvalue_2 (Transformation|GetActorForwardVector _owneractor_2))
  (bind _returnvalue_3 (* _returnvalue_2 5e+01))
  (bind _returnvalue_4 (+ _returnvalue _returnvalue_3))
  (if (not (CallFunction|FHasCooldown))
    (bind _returnvalue_5 (Collision|SphereTraceByChannel _returnvalue_4 (- _returnvalue_4 "0.000000,0.000000,100.000000") 3e+01 "TraceTypeQuery1" false 0 "None"))
    (if _returnvalue_5
      (|CallParentFunction)
      (bind _returnvalue_6 (Game|SpawnActorfromClass "/Script/Engine.StaticMeshActor" (Math|Transform|MakeTransform (+ (Transformation|GetActorLocation _owneractor) (* (Transformation|GetActorForwardVector _owneractor) 1.5e+02) "0.000000,0.000000,-200.000000") (Math|Rotator|CombineRotators (Transformation|GetActorRotation _owneractor) "0.000000,90.000000,0.000000") "1.000000,1.000000,1.000000") "Undefined" "MultiplyWithRoot" 0 0))
      (Transformation|SetMobility _returnvalue_6 "Movable")
      (Components|StaticMesh|SetStaticMesh (Variables|/Script/Engine.StaticMeshActor|GetStaticMeshComponent _returnvalue_6) "/Game/Shota/Assets/Meshes/Rock/Boulder/Rock1_Nanite.Rock1_Nanite")
      (Variables|Default|SetStepCount 0)
      (Pawn|Components|CharacterMovement|SetMovementMode (Variables|/Script/Engine.Character|GetCharacterMovement (Variables|Default|GetOwnerActor)) "MOVE_None" 0)
      (bind _returnvalue_7 (Utilities|Time|SetTimerbyEvent (delegate Custom|MoveUpStep) 0.02 true))
      (Utilities|FlowControl|Delay 3.0)
      (bind _size (Timeline|DieOut PlayFromStart)
        (:Update
          (Transformation|SetActorScale3D _returnvalue_6 (Math|Conversions|ToVector(Float) _size)))
        (:Finished
          (Actor|DestroyActor _returnvalue_6))))))

(fn ConstructionScript
  (|CallParentFunction))