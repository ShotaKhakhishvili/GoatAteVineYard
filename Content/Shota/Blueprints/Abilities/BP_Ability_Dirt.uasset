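; Dirt ability for a character, with a rock-raising main ability and a dirt-throw simple ability, both cooldown-gated; it applies the ABP_Dirt anim class on BeginPlay.
; The main ability requires ground ahead, then spawns a rock below it, freezing movement while a looping timer steps it upward; a timeline later scales and destroys it.
; The simple ability launches the character and, after a short montage delay, spawns an actor at MeleeSocket with hit sounds.
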(event Custom|MoveUpStep
  (bind _lastspawnedmesh (Variables|Default|GetLastSpawnedMesh))
  (Utilities|IsValid _lastspawnedmesh
    (:Is%20Valid
      (Transformation|AddActorWorldOffset _lastspawnedmesh "0.000000,0.000000,4.000000")
      (bind _result (Math|Integer|IncrementInt (Variables|Default|GetStepCount))
        (:%20%20
          (if (> _result 25)
            (Utilities|Time|ClearandInvalidateTimerbyHandle (Variables|Default|GetMoveUpEventHandle))
            (Pawn|Components|CharacterMovement|SetMovementMode (Variables|/Script/Engine.Character|GetCharacterMovement (Variables|Default|GetOwnerActor)) "MOVE_Walking" 0)))))))

(event EventActivateSimpleAbility
  (if (not (CallFunction|FHasCooldownorFallingS))
    (|CallParentFunction)
    (CallFunction|FLaunchCharacter 5e+02 5e+01)
    (Animation|Montage|PlayMontage (Variables|/Script/Engine.Character|GetMesh (Variables|Default|GetOwnerActor)) "/Game/Gigi/NewCharacters/Dirt/Dirt_Throw_dirt_Montage.Dirt_Throw_dirt_Montage"
      (:then
        (Utilities|FlowControl|Delay 0.28)
        (Game|SpawnActorfromClass "/Game/Shota/Blueprints/AbilityDamagers/BP_AbilityDamager_Melee.BP_AbilityDamager_Melee_C" (Transformation|GetSocketTransform (Variables|/Script/Engine.Character|GetMesh (Variables|Default|GetOwnerActor)) "MeleeSocket" "RTS_World") "Undefined" "MultiplyWithRoot" 0 self (Variables|Default|GetSimpleAbilityHitSounds) 0)))))

(event EventBeginPlay
  (|CallParentFunction)
  (Components|SkeletalMesh|SetAnimInstanceClass (Variables|/Script/Engine.Character|GetMesh (Variables|Default|GetOwnerActor)) "/Game/Gigi/NewCharacters/ABPS/ABP_Dirt.ABP_Dirt_C"))

(event EventActivateAbility
  (bind _owneractor (Variables|Default|GetOwnerActor))
  (bind _owneractor_2 (Variables|Default|GetOwnerActor))
  (bind _returnvalue (Transformation|GetActorLocation _owneractor_2))
  (bind _returnvalue_2 (Transformation|GetActorForwardVector _owneractor_2))
  (bind _returnvalue_3 (* _returnvalue_2 5e+01))
  (bind _returnvalue_4 (+ _returnvalue _returnvalue_3))
  (if (not (CallFunction|FHasCooldown))
    (bind _returnvalue_5 (Collision|SphereTraceByChannel _returnvalue_4 (- _returnvalue_4 "0.000000,0.000000,100.000000") 3e+01 "TraceTypeQuery1" false 0 "None"))
    (if _returnvalue_5
      (|CallParentFunction)
      (Animation|Montage|PlayMontage (Variables|/Script/Engine.Character|GetMesh (Variables|Default|GetOwnerActor)) "/Game/Gigi/NewCharacters/Dirt/Dirt_pull_Ground_Montage1.Dirt_pull_Ground_Montage1"
        (:then
          (bind _returnvalue_6 (Game|SpawnActorfromClass "/Script/Engine.StaticMeshActor" (Math|Transform|MakeTransform (+ (Transformation|GetActorLocation _owneractor) (* (Transformation|GetActorForwardVector _owneractor) 1.5e+02) "0.000000,0.000000,-200.000000") (Math|Rotator|CombineRotators (Transformation|GetActorRotation _owneractor) "0.000000,90.000000,0.000000") "1.000000,1.000000,1.000000") "Undefined" "MultiplyWithRoot" 0 0))
          (Variables|Default|SetLastSpawnedMesh _returnvalue_6)
          (Transformation|SetMobility (Variables|Default|GetLastSpawnedMesh) "Movable")
          (Components|StaticMesh|SetStaticMesh (Variables|/Script/Engine.StaticMeshActor|GetStaticMeshComponent (Variables|Default|GetLastSpawnedMesh)) "/Game/Shota/Assets/Meshes/Rock/Boulder/Rock1_Nanite.Rock1_Nanite")
          (Variables|Default|SetStepCount 0)
          (Pawn|Components|CharacterMovement|SetMovementMode (Variables|/Script/Engine.Character|GetCharacterMovement (Variables|Default|GetOwnerActor)) "MOVE_None" 0)
          (bind _returnvalue_7 (Utilities|Time|SetTimerbyEvent (delegate Custom|MoveUpStep) 0.02 true))
          (Variables|Default|SetMoveUpEventHandle _returnvalue_7)
          (Utilities|FlowControl|Delay 3.0)
          (bind _size (Timeline|DieOut PlayFromStart)
            (:Update
              (Transformation|SetActorScale3D (Variables|Default|GetLastSpawnedMesh) (Math|Conversions|ToVector(Float) _size)))
            (:Finished
              (Actor|DestroyActor (Variables|Default|GetLastSpawnedMesh))
              (Variables|Default|SetLastSpawnedMesh 0)
              (if (Utilities|Time|IsValidTimerHandle (Variables|Default|GetMoveUpEventHandle))
                (Utilities|Time|ClearandInvalidateTimerbyHandle (Variables|Default|GetMoveUpEventHandle))))))))))

(fn ConstructionScript
  (|CallParentFunction))