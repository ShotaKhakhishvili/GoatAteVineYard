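; Gun ability Blueprint that gives its owning actor a gun moveset, switching the owner's mesh to the ABP_Gun anim instance on BeginPlay.
; The main ability, gated by cooldown, spawns a GunBomb damager above the owner.
; The simple ability, blocked by cooldown or falling, spawns a melee damager ahead of the owner and plays a headshot montage.
; Both pass themselves as the damager's owning ability and call the parent activation.
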(event EventActivateSimpleAbility
  (bind _owneractor (Variables|Default|GetOwnerActor))
  (bind _returnvalue (Transformation|GetActorTransform _owneractor))
  (if (not (CallFunction|FHasCooldownorFallingS))
    (Development|PrintString "dd")
    (Game|SpawnActorfromClass "/Game/Shota/Blueprints/AbilityDamagers/BP_AbilityDamager_Melee.BP_AbilityDamager_Melee_C" (Math|Transform|MakeTransform (+ (.location _returnvalue) "0.000000,0.000000,50.000000" (* (Transformation|GetActorForwardVector _owneractor) 5e+01)) (.rotation _returnvalue) (.scale _returnvalue)) "Undefined" "MultiplyWithRoot" 0 self 0)
    (|CallParentFunction)
    (Animation|Montage|PlayMontage (Variables|/Script/Engine.Character|GetMesh (Variables|Default|GetOwnerActor)) "/Game/Shota/Assets/Things/Gun/AM_Headhshot.AM_Headhshot")))

(event EventBeginPlay
  (|CallParentFunction)
  (Components|SkeletalMesh|SetAnimInstanceClass (Variables|/Script/Engine.Character|GetMesh (Variables|Default|GetOwnerActor)) "/Game/Shota/Blueprints/Fighter/ABPS/ABP_Gun.ABP_Gun_C"))

(event EventActivateAbility
  (bind _owneractor (Variables|Default|GetOwnerActor))
  (bind _returnvalue (Transformation|GetActorTransform _owneractor))
  (if (not (CallFunction|FHasCooldown))
    (Game|SpawnActorfromClass "/Game/Shota/Blueprints/AbilityDamagers/BP_AbilityDamager_GunBomb.BP_AbilityDamager_GunBomb_C" (Math|Transform|MakeTransform (+ (.location _returnvalue) "0.000000,0.000000,150.000000") "90.000000,0.000000,0.000000" (.scale _returnvalue)) "Undefined" "MultiplyWithRoot" 0 self 0)
    (|CallParentFunction)))

(fn ConstructionScript
  (|CallParentFunction))