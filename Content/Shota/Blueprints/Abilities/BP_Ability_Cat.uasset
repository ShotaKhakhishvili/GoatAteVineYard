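; BP_Ability_Cat is the cat ability set, applying the cat anim class to the owner's mesh on BeginPlay.
; The main ability, gated by cooldown, launches the character in a strong leap.
; The simple ability, gated by a cooldown-or-falling check, does a short lunge with a punch montage, then spawns a melee damager in front of the owner after a brief delay.
; An unconnected delayed reset to Walking never runs.
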(event EventActivateSimpleAbility
  (bind _owneractor (Variables|Default|GetOwnerActor))
  (bind _returnvalue (Transformation|GetActorTransform _owneractor))
  (if (not (CallFunction|FHasCooldownorFallingS))
    (|CallParentFunction)
    (CallFunction|FLaunchCharacter 5e+02 5e+01)
    (Animation|Montage|PlayMontage (Variables|/Script/Engine.Character|GetMesh (Variables|Default|GetOwnerActor)) "/Game/Shota/Assets/Things/Cat/NewOnes/AM_CatPunch.AM_CatPunch"
      (:then
        (Utilities|FlowControl|Delay 0.2)
        (Game|SpawnActorfromClass "/Game/Shota/Blueprints/AbilityDamagers/BP_AbilityDamager_Melee.BP_AbilityDamager_Melee_C" (Math|Transform|MakeTransform (+ (.location _returnvalue) "0.000000,0.000000,50.000000" (* (Transformation|GetActorForwardVector _owneractor) 5e+01)) (.rotation _returnvalue) (.scale _returnvalue)) "Undefined" "MultiplyWithRoot" 0 self 0)))))

(event EventBeginPlay
  (|CallParentFunction)
  (Components|SkeletalMesh|SetAnimInstanceClass (Variables|/Script/Engine.Character|GetMesh (Variables|Default|GetOwnerActor)) "/Game/Shota/Blueprints/Fighter/ABPS/ABP_Cat.ABP_Cat_C"))

(event EventActivateAbility
  (if (not (CallFunction|FHasCooldown))
    (|CallParentFunction)
    (CallFunction|FLaunchCharacter 2e+03 5e+02)))

(fn ConstructionScript
  (|CallParentFunction))