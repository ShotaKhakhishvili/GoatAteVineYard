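; BP_DroppedLoot is a pickup that spins and bobs in place, showing its material on a plane.
; When the player pawn overlaps its sphere, it starts following, interpolating toward the player every tick.
; Once within close range, it notifies BP_FighterCharacter_Player that the droppable was received, spawns a pickup Niagara effect at the player, and destroys itself.
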(event OnComponentBeginOverlap(Sphere)
  (params (OverlappedComponent :type Primitive%20Component%20Object%20Reference) (OtherActor :type Actor%20Object%20Reference) (OtherComp :type Primitive%20Component%20Object%20Reference) (OtherBodyIndex :type Integer) (bFromSweep :type Boolean) (SweepResult :type Hit%20Result%20Structure%20%28by%20ref%29))
  (if (== OtherActor (Game|Player|GetPlayerPawn 0))
    (Variables|Default|SetFollowingPlayer true)))

(event EventTick
  (params (DeltaSeconds :type Float%20%28single-precision%29))
  (Transformation|AddRelativeRotation (Variables|Default|GetPlane) (Math|Rotator|MakeRotator 0.0 0.0 (* DeltaSeconds 25.0)) false false)
  (Transformation|SetRelativeLocation (Variables|Default|GetPlane) (Math|Vector|MakeVector 0.0 0.0 (* (Math|Trig|Sin(Radians) (* (Actor|GetGameTimeSinceCreation) 3.0)) 5e+01)) false false)
  (if (Variables|Default|GetFollowingPlayer)
    (Transformation|SetActorLocation (Math|Interpolation|VInterpTo (Transformation|GetActorLocation) (Transformation|GetActorLocation (Game|Player|GetPlayerPawn 0)) (Utilities|Time|GetWorldDeltaSeconds) 3.0) false false)
    (if (<= (Math|Vector|Distance(Vector) (Transformation|GetActorLocation) (Transformation|GetActorLocation (Game|Player|GetPlayerPawn 0))) 4e+01)
      (bind _asbp_fighter_character_player (Utilities|Casting|CastToBP_FighterCharacter_Player (Game|Player|GetPlayerPawn 0)))
      (Default|CallDroppableReceived _asbp_fighter_character_player)
      (Niagara|SpawnSystematLocation "/Game/NiagaraExamples/FX_PickUp/NS_Pickup_Timeout.NS_Pickup_Timeout" (Transformation|GetActorLocation _asbp_fighter_character_player) "0, 0, 0" "2.000000,2.000000,2.000000")
      (Actor|DestroyActor))))

(event EventBeginPlay
  (Rendering|Material|SetMaterial (Variables|Default|GetPlane) 0 (Variables|Default|GetMaterial)))

(fn ConstructionScript)