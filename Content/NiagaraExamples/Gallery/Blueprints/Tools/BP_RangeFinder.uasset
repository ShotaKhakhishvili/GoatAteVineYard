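; BP_RangeFinder is a Niagara Examples gallery tool actor that displays how far the player camera is from it.
; Every Tick it takes the length of the vector between its scene root and player 0's camera manager location.
; It rounds that distance to a whole number, appends "cm" and writes it to a TextRender component.
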(event EventBeginPlay)

(event Collision|EventActorBeginOverlap
  (params (OtherActor :type Actor%20Object%20Reference)))

(event EventTick
  (params (DeltaSeconds :type Float%20%28single-precision%29))
  (Rendering|Components|TextRender|SetText (Variables|Default|GetTextRender) (Utilities|Text|ToText(String) (Utilities|String|Append (Utilities|String|ToString(Integer) (Math|Float|Round (Math|Vector|VectorLength (- (Transformation|GetWorldLocation (Variables|Default|GetDefaultSceneRoot)) (Camera|GetCameraLocation (Game|GetPlayerCameraManager 0)))))) "cm"))))

(fn ConstructionScript)